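; BP_Trap is a spike trap that hits any BP_ThirdPersonCharacter overlapping the actor.
; After an initial SpikeUpTime delay, a timeline drives the Spike component's relative height between rest and raised positions, restarting itself on finish to loop indefinitely.
; Actor overlap calls GotHit on the character, passing the trap, with no check on the spike's current position.
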(event `self.ReceiveBeginPlay`
  (`KismetSystemLibrary.Delay` (`self.SpikeUpTime`))
  (`self.SpikeTrap Working`))

(event `SpikeTrap Working`
  (bind (_direction _alpha) (`Timeline|Timeline_Loop` :`NewTime` (`self.SpikeUpTime`) :!via `PlayFromStart`)
    (:`Update`
      (`SceneComponent.K2_SetRelativeLocation` (`self.Spike`) (`KismetMathLibrary.VLerp` (0.0 0.0 0.0) (0.0 0.0 85.0) _alpha) false false))
    (:`Finished`
      (`self.SpikeTrap Working`))))

(event `self.ReceiveActorBeginOverlap`
  (params (OtherActor :type "Actor Object Reference"))
  (bind _asbp_third_person_character (cast `/Game/Characters/PlayerCharacter/BP_ThirdPersonCharacter` OtherActor))
  (`/Game/Characters/PlayerCharacter/BP_ThirdPersonCharacter.GotHit` _asbp_third_person_character self))

(fn `UserConstructionScript`)