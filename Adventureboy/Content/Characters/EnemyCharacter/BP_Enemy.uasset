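; BP_Enemy is an enemy character that wanders and drops a coin when defeated.
; From BeginPlay it moves to random navigable points within a radius of itself, pausing after each successful move before picking another.
; Its Defeated event runs once, stopping movement, playing a death montage and launching the enemy up and away from the player.
; A timeline then shrinks it to nothing before it spawns BP_Coin and destroys itself.
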(event `self.ReceiveBeginPlay`
  (`self.Move Around`))

(event `Move Around`
  ; AI Move around
  (bind _randomlocation (`NavigationSystemV1.K2_GetRandomLocationInNavigableRadius` (`self.K2_GetActorLocation`) 500.0 null null))
  (`|AIMoveTo` self _randomlocation null
    (:`OnSuccess`
      (`KismetSystemLibrary.Delay` 2.0)
      (`self.Move Around`))))

(event `Defeated`
  ; Defeated
  (`/Engine/EditorBlueprintResources/StandardMacros.DoOnce` false
    (:`Completed`
      (`Controller.StopMovement` (`AIBlueprintHelperLibrary.GetAIController` self))
      (`|PlayMontage` (`self.Mesh`) "/Game/Characters/EnemyCharacter/Animations/Enemy_Anim_MonsterArmature_Death_Montage.Enemy_Anim_MonsterArmature_Death_Montage"
        (:`then`
          (`self.LaunchCharacter` (* (`KismetMathLibrary.MakeVector` (.x (`KismetMathLibrary.GetDirectionUnitVector` (`self.K2_GetActorLocation` (`GameplayStatics.GetPlayerCharacter` 0)) (`self.K2_GetActorLocation`))) (.y (`KismetMathLibrary.GetDirectionUnitVector` (`self.K2_GetActorLocation` (`GameplayStatics.GetPlayerCharacter` 0)) (`self.K2_GetActorLocation`))) 0.5) 500.0) true true)
          (`KismetSystemLibrary.Delay` 0.45)
          (bind (_direction _alpha) (`Timeline|Timeline_Defeated`)
            (:`Update`
              (`self.SetActorScale3D` (`KismetMathLibrary.VLerp` (1.0 1.0 1.0) (0.0 0.0 0.0) _alpha)))
            (:`Finished`
              (`|SpawnActorFromClass` "/Game/Items/Coin/BP_Coin.BP_Coin_C" (`KismetMathLibrary.MakeTransform` (`KismetMathLibrary.MakeVector` (.x (`self.K2_GetActorLocation`)) (.y (`self.K2_GetActorLocation`)) 70.0)) "Undefined" "MultiplyWithRoot" null null)
              (`self.K2_DestroyActor`))))))))

(fn `UserConstructionScript`)