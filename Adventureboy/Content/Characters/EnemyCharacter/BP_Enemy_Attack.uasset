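; Enemy character that roams, chases the player on sight and attacks on contact.
; It wanders to random nearby navmesh points until a detection collider overlap starts a repeating AI MoveTo chase, returning to wandering when the overlap ends.
; Hit collider overlaps play a montage and call GotHit on the player.
; Defeated disables hits, plays a death montage, launches it away from the player, shrinks it by timeline, then spawns a coin and destroys it.
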(event `self.ReceiveBeginPlay`
  (`self.Move Around`))

(event `Move Around`
  ; AI Move around
  (bind _randomlocation (`NavigationSystemV1.K2_GetRandomLocationInNavigableRadius` (`self.K2_GetActorLocation`) 500.0 null null))
  (`|AIMoveTo` self _randomlocation null
    (:`OnSuccess`
      (`KismetSystemLibrary.Delay` 1.0)
      (set `self.Is Seeing Player?` (not (`self.Is Seeing Player?`)))
      (`self.Move Around`))))

(event `ChasePlayer`
  ; Chase Player
  (`AITask_MoveTo.AIMoveTo` (`AIBlueprintHelperLibrary.GetAIController` self) (0.0 0.0 0.0) (`self.Player`)
    (:`OnRequestFailed`
      _)
    (:`OnMoveFinished`
      _))
  (`KismetSystemLibrary.Delay` 1.0)
  (if (`self.Is Seeing Player?`)
    (`self.ChasePlayer`)
    (else
      (`self.Move Around`))))

(event `Defeated`
  ; Defeated
  (`/Engine/EditorBlueprintResources/StandardMacros.DoOnce` false
    (:`Completed`
      (`PrimitiveComponent.SetCollisionEnabled` (`self.HitCollision`) "NoCollision")
      (`Controller.StopMovement` (`AIBlueprintHelperLibrary.GetAIController` self))
      (`|PlayMontage` (`self.Mesh`) "/Game/Characters/EnemyCharacter/Animations/Enemy_Anim_MonsterArmature_Death_Montage.Enemy_Anim_MonsterArmature_Death_Montage"
        (:`then`
          (`self.LaunchCharacter` (* (`KismetMathLibrary.MakeVector` (.x (`KismetMathLibrary.GetDirectionUnitVector` (`self.K2_GetActorLocation` (`GameplayStatics.GetPlayerCharacter` 0)) (`self.K2_GetActorLocation`))) (.y (`KismetMathLibrary.GetDirectionUnitVector` (`self.K2_GetActorLocation` (`GameplayStatics.GetPlayerCharacter` 0)) (`self.K2_GetActorLocation`))) 0.5) 500.0) true true)
          (`KismetSystemLibrary.Delay` 0.45)
          (bind (_direction _alpha) (`Timeline|Timeline_Defeated`)
            (:`Update`
              (`self.SetActorScale3D` (`KismetMathLibrary.VLerp` (1.0 1.0 1.0) (0.0 0.0 0.0) _alpha)))
            (:`Finished`
              (`|SpawnActorFromClass` "/Game/Items/Coin/BP_Coin.BP_Coin_C" (`KismetMathLibrary.MakeTransform` (`KismetMathLibrary.MakeVector` (.x (`self.K2_GetActorLocation`)) (.y (`self.K2_GetActorLocation`)) 70.0)) "Undefined" "MultiplyWithRoot" null null)
              (`self.K2_DestroyActor`))))))))

(event `self.DetetctionCollision.OnComponentBeginOverlap`
  (params (OverlappedComponent :type "PrimitiveComponent Object Reference") (OtherActor :type "Actor Object Reference") (OtherComp :type "PrimitiveComponent Object Reference") (OtherBodyIndex :type Integer) (bFromSweep :type Boolean) (SweepResult :type "HitResult Structure (by ref)"))
  ; See Player
  (bind _asbp_third_person_character (cast `/Game/Characters/PlayerCharacter/BP_ThirdPersonCharacter` OtherActor))
  (set `self.Player` _asbp_third_person_character)
  (set `self.Is Seeing Player?` true)
  (`self.ChasePlayer`))

(event `self.DetetctionCollision.OnComponentEndOverlap`
  (params (OverlappedComponent :type "PrimitiveComponent Object Reference") (OtherActor :type "Actor Object Reference") (OtherComp :type "PrimitiveComponent Object Reference") (OtherBodyIndex :type Integer))
  ; Unseen Player
  (cast `/Game/Characters/PlayerCharacter/BP_ThirdPersonCharacter` OtherActor)
  (set `self.Is Seeing Player?` false)
  (`self.Move Around`))

(event `self.HitCollision.OnComponentBeginOverlap`
  (params (OverlappedComponent :type "PrimitiveComponent Object Reference") (OtherActor :type "Actor Object Reference") (OtherComp :type "PrimitiveComponent Object Reference") (OtherBodyIndex :type Integer) (bFromSweep :type Boolean) (SweepResult :type "HitResult Structure (by ref)"))
  ; Hit Player
  (`self.PlayAnimMontage` "/Game/Characters/EnemyCharacter/Animations/AM_Hit.AM_Hit")
  (bind _asbp_third_person_character (cast `/Game/Characters/PlayerCharacter/BP_ThirdPersonCharacter` OtherActor))
  (`/Game/Characters/PlayerCharacter/BP_ThirdPersonCharacter.GotHit` _asbp_third_person_character self))

(fn `UserConstructionScript`)